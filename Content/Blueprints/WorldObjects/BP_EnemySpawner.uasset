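; BP_EnemySpawner is a world object that spawns BP_Enemy actors inside a configurable box volume.
; On BeginPlay it starts a timer that fires once or repeats on an interval, depending on OneShot.
; Each tick of the timer spawns a random count within a min-max range, each at a random point in the box.
; The construction script sizes the box from the Size variable.
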(event `self.ReceiveBeginPlay`
  (`KismetSystemLibrary.K2_SetTimerDelegate` (delegate `SpawnEnemies`) (`self.Interval`) (not (`self.OneShot`))))

(event `SpawnEnemies`
  (bind _box (`self.Box`))
  (for _ (range (+ (`KismetMathLibrary.RandomIntegerInRange` (`self.AmountToSpawnMin`) (`self.AmountToSpawnMax`)) 1))
    (`|SpawnActorFromClass` "/Game/Blueprints/Enemies/BP_Enemy.BP_Enemy_C" (`KismetMathLibrary.MakeTransform` (`KismetMathLibrary.RandomPointInBoundingBox` (`SceneComponent.K2_GetComponentLocation` _box) (`BoxComponent.BoxExtent` _box))) "Undefined" "MultiplyWithRoot" null null)))

(fn `UserConstructionScript`
  (`BoxComponent.SetBoxExtent` (`self.Box`) (`self.Size`) true))