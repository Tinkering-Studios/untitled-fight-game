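; BP_MainGameMode is the main game mode that sets up the player's HUD when play begins.
; On BeginPlay it creates a WBP_Base root widget, stores it as HUD, adds it to the viewport and pushes WBP_GameHUD onto its MainStack.
; It then switches the first player controller to game-only input with the cursor hidden, and exposes the root widget through GetHUDBase.
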(event `self.ReceiveBeginPlay`
  (bind _returnvalue (`GameplayStatics.GetPlayerController` 0))
  (bind _returnvalue_2 (`|CreateWidget` "/Game/Blueprints/UI/Core/WBP_Base.WBP_Base_C"))
  (bind _output_get (set `self.HUD` _returnvalue_2))
  (`UserWidget.AddToViewport` _output_get 0)
  (`CommonActivatableWidgetContainerBase.BP_AddWidget` (`/Game/Blueprints/UI/Core/WBP_Base.MainStack` _output_get) "/Game/Blueprints/UI/Game/WBP_GameHUD.WBP_GameHUD_C")
  (`WidgetBlueprintLibrary.SetInputMode_GameOnly` _returnvalue true)
  (set `PlayerController.bShowMouseCursor` false _returnvalue))

(fn `GetHUDBase`
  (returns (WBP_Base :type "/Game/Blueprints/UI/Core/WBP_Base Object Reference"))
  (return (`self.HUD`)))

(fn `UserConstructionScript`)