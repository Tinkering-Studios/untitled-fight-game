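; Player character for a melee brawler with left/right light and heavy punches, kicks, and throwable held weapons.
; Controller events and input drive capsule traces, deduplicated per actor, into ProcessHit, which applies typed damage, doubled during Rage events.
; Enemy hits build temporary score and combo (points double during DoublePoints), banked as their product when the combo timer expires.
; Also handles pickup highlighting, pause and death screens, and difficulty-dependent delayed health regeneration.
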(event `self.ReceiveBeginPlay`
  (bind _asmain_controller (cast `MainController` (`GameplayStatics.GetPlayerController` 0)))
  (add `MainController.OnLightAttack` _asmain_controller (`|CreateDelegate` :!event `LightAttack`))
  (add `MainController.OnHeavyAttack` _asmain_controller (`|CreateDelegate` :!event `HeavyAttack`))
  (add `self.OnEnemyHit` (`|CreateDelegate` :!event `EnemyHit`)))

(event `LightAttack`
  (params (IsRight :type Boolean))
  (bind _returnvalue (`SceneComponent.K2_GetComponentLocation` (`self.ChestCentre1`)))
  (bind _returnvalue_2 (`SceneComponent.K2_GetComponentLocation` (`self.ChestCentre2`)))
  (bind _array (`|MakeArray` (`ChildActorComponent.ChildActor` (`self.RightHandThrowable`)) (`ChildActorComponent.ChildActor` (`self.LeftHandThrowable`))))
  ;[1 1 1] Rewrite this soon
  (if IsRight
    (bind _hasrightweapon (`self.HaveRightWeapon`))
    (if _hasrightweapon
      (`self.ThrowWeapon` true)
      (else
        (bind _outhits (`KismetSystemLibrary.CapsuleTraceMulti` _returnvalue (+ _returnvalue (* (`self.GetActorForwardVector`) 80.0)) 50.0 50.0 "TraceTypeQuery1" false _array))
        (`ActionManager.ExecuteAction` (`self.ActionsManager`) (struct :`TagName` "Action.LightRight"))
        (bind _results (`self.CorrectlyFilterHits` _outhits))
        (if (> (`KismetArrayLibrary.Array_Length` _results) 0)
          (`GameplayStatics.PlaySoundAtLocation` "/Game/Sounds/SC_Punch.SC_Punch" (`self.K2_GetActorLocation`) (struct) 1.0 1.0 0.0 null null null null))
        (for _array_element _results
          (`self.ProcessHit` _array_element))))
    (else
      (bind _hasleftweapon (`self.HaveLeftWeapon`))
      (if _hasleftweapon
        (`self.ThrowWeapon` false)
        (else
          (bind _outhits_2 (`KismetSystemLibrary.CapsuleTraceMulti` _returnvalue_2 (+ _returnvalue_2 (* (`self.GetActorForwardVector`) 80.0)) 50.0 50.0 "TraceTypeQuery1" false _array))
          (`ActionManager.ExecuteAction` (`self.ActionsManager`) (struct :`TagName` "Action.LightLeft"))
          (bind _results_2 (`self.CorrectlyFilterHits` _outhits_2))
          (if (> (`KismetArrayLibrary.Array_Length` _results_2) 0)
            (`GameplayStatics.PlaySoundAtLocation` "/Game/Sounds/SC_Punch.SC_Punch" (`self.K2_GetActorLocation`) (struct) 1.0 1.0 0.0 null null null null))
          (for _array_element_2 _results_2
            (`self.ProcessHit` _array_element_2)))))))

(event `HeavyAttack`
  (params (IsRight :type Boolean))
  (bind _returnvalue (`SceneComponent.K2_GetComponentLocation` (`self.ChestCentre1`)))
  (bind _returnvalue_2 (`SceneComponent.K2_GetComponentLocation` (`self.ChestCentre2`)))
  (bind _array (`|MakeArray` (`ChildActorComponent.ChildActor` (`self.RightHandThrowable`)) (`ChildActorComponent.ChildActor` (`self.LeftHandThrowable`))))
  ;[1 1 1] Rewrite this soon
  (if IsRight
    (bind _outhits (`KismetSystemLibrary.CapsuleTraceMulti` _returnvalue (+ _returnvalue (* (`SceneComponent.GetForwardVector` (`self.Camera`)) 80.0)) 50.0 50.0 "TraceTypeQuery1" false _array))
    (`ActionManager.ExecuteAction` (`self.ActionsManager`) (struct :`TagName` "Action.HeavyRight"))
    (bind _results (`self.CorrectlyFilterHits` _outhits))
    (if (> (`KismetArrayLibrary.Array_Length` _results) 0)
      (`GameplayStatics.PlaySoundAtLocation` "/Game/Sounds/SC_Punch.SC_Punch" (`self.K2_GetActorLocation`) (struct) 1.0 1.0 0.0 null null null null))
    (for _array_element _results
      (`self.ProcessHit` _array_element true))
    (else
      (bind _outhits_2 (`KismetSystemLibrary.CapsuleTraceMulti` _returnvalue_2 (+ _returnvalue_2 (* (`SceneComponent.GetForwardVector` (`self.Camera`)) 80.0)) 50.0 50.0 "TraceTypeQuery1" false _array))
      (`ActionManager.ExecuteAction` (`self.ActionsManager`) (struct :`TagName` "Action.HeavyLeft"))
      (bind _results_2 (`self.CorrectlyFilterHits` _outhits_2))
      (if (> (`KismetArrayLibrary.Array_Length` _results_2) 0)
        (`GameplayStatics.PlaySoundAtLocation` "/Game/Sounds/SC_Punch.SC_Punch" (`self.K2_GetActorLocation`) (struct) 1.0 1.0 0.0 null null null null))
      (for _array_element_2 _results_2
        (`self.ProcessHit` _array_element_2 true)))))

(event `EnemyHit` :!signature `self.OnEnemyHit`
  (params (AttackType :type "EAttackType Enum" :default "LightAttack"))
  (bind _statscomponent (`self.StatsComponent`))
  (`StatisticsComponent.ModifyCurrentValueOfStatistic` _statscomponent (struct :`TagName` "Misc.TempPoint") (`KismetMathLibrary.SelectFloat` 200.0 100.0 (`EventsManager.IsEventActive` (`self.GetComponentByClass` (`GameplayStatics.GetGameMode`) "/Script/untitledfightgame.EventsManager") (`BlueprintGameplayTagLibrary.MakeLiteralGameplayTag` (struct :`TagName` "Events.DoublePoints")))))
  (`StatisticsComponent.ModifyCurrentValueOfStatistic` _statscomponent (struct :`TagName` "Misc.Combo") 1.0)
  (`KismetSystemLibrary.K2_ClearAndInvalidateTimerHandle` (`self.CurrentComboTimer`))
  (bind _returnvalue (`KismetSystemLibrary.K2_SetTimerDelegate` (delegate `CustomEvent`) 3.0))
  (set `self.CurrentComboTimer` _returnvalue)
  (bind _wbp_base (message `/Game/Blueprints/Interfaces/BPI_HUD.GetHUDBase` (`GameplayStatics.GetGameMode`)))
  (bind _aswbp_game_hud (cast `/Game/Blueprints/UI/Game/WBP_GameHUD` (`CommonActivatableWidgetContainerBase.GetActiveWidget` (`/Game/Blueprints/UI/Core/WBP_Base.MainStack` _wbp_base))))
  (bind _wbp_combocounter (`/Game/Blueprints/UI/Game/WBP_GameHUD.WBP_ComboCounter` _aswbp_game_hud))
  (`Widget.SetVisibility` _wbp_combocounter "SelfHitTestInvisible")
  (`Widget.SetVisibility` (`/Game/Blueprints/UI/Game/WBP_GameHUD.TempScoreMeter` _aswbp_game_hud) "SelfHitTestInvisible")
  (bind _tempscoremeter (`/Game/Blueprints/UI/Game/WBP_GameHUD.TempScoreMeter` _aswbp_game_hud))
  (`Widget.SetRenderOpacity` _tempscoremeter 1.0)
  (`Widget.SetRenderTranslation` _tempscoremeter (0.0 0.0))
  (`/Game/Blueprints/UI/Game/WBP_ComboCounter.RestartFade` _wbp_combocounter))

(event `CustomEvent`
  (bind _statscomponent (`self.StatsComponent`))
  (bind _returnvalue_currentvalue (break `StatisticInformation` (`StatisticsComponent.GetStatInfoByTag` _statscomponent (struct :`TagName` "Misc.Combo"))))
  (bind _returnvalue_currentvalue_2 (break `StatisticInformation` (`StatisticsComponent.GetStatInfoByTag` _statscomponent (struct :`TagName` "Misc.TempPoint"))))
  (bind _wbp_base (message `/Game/Blueprints/Interfaces/BPI_HUD.GetHUDBase` (`GameplayStatics.GetGameMode`)))
  (bind _aswbp_game_hud (cast `/Game/Blueprints/UI/Game/WBP_GameHUD` (`CommonActivatableWidgetContainerBase.GetActiveWidget` (`/Game/Blueprints/UI/Core/WBP_Base.MainStack` _wbp_base))))
  (`/Game/Blueprints/UI/Game/WBP_GameHUD.PointsAdded` _aswbp_game_hud)
  (`Widget.SetVisibility` (`/Game/Blueprints/UI/Game/WBP_GameHUD.WBP_ComboCounter` _aswbp_game_hud) "Hidden")
  (`StatisticsComponent.ModifyCurrentValueOfStatistic` _statscomponent (struct :`TagName` "Misc.Points") (* _returnvalue_currentvalue_2 _returnvalue_currentvalue))
  (`StatisticsComponent.SetCurrentValueOfStatistic` _statscomponent (struct :`TagName` "Misc.Combo") 0.0)
  (`StatisticsComponent.SetCurrentValueOfStatistic` _statscomponent (struct :`TagName` "Misc.TempPoint") 0.0))

(event `EnhancedInput|/Game/Data/Input/IA_Pause`
  (params (ActionValue :type Boolean) (ElapsedSeconds :type "Float (double-precision)") (TriggeredSeconds :type "Float (double-precision)") (InputAction :type "InputAction Object Reference" :default "/Game/Data/Input/IA_Pause.IA_Pause"))
  (bind _returnvalue (`GameplayStatics.GetPlayerController` 0))
  (bind _returnvalue_2 (`GameplayStatics.GetPlayerController` 0))
  (:`Triggered`
    (if (`GameplayStatics.IsGamePaused`)
      (`GameplayStatics.SetGamePaused` false)
      (bind _foundwidgets (`WidgetBlueprintLibrary.GetAllWidgetsOfClass` "/Game/Blueprints/UI/Core/WBP_Base.WBP_Base_C"))
      (`CommonActivatableWidget.DeactivateWidget` (`CommonActivatableWidgetContainerBase.GetActiveWidget` (`/Game/Blueprints/UI/Core/WBP_Base.PauseStack` (`|GetArrayItem` _foundwidgets))))
      (`WidgetBlueprintLibrary.SetInputMode_GameOnly` _returnvalue_2 true)
      (set `PlayerController.bShowMouseCursor` false _returnvalue_2)
      (else
        (`GameplayStatics.SetGamePaused` true)
        (bind _foundwidgets_2 (`WidgetBlueprintLibrary.GetAllWidgetsOfClass` "/Game/Blueprints/UI/Core/WBP_Base.WBP_Base_C"))
        (bind _output (`|GetArrayItem` _foundwidgets_2))
        (`CommonActivatableWidgetContainerBase.BP_AddWidget` (`/Game/Blueprints/UI/Core/WBP_Base.PauseStack` _output) "/Game/Blueprints/UI/Game/WBP_Pause.WBP_Pause_C")
        (`WidgetBlueprintLibrary.SetInputMode_GameAndUIEx` _returnvalue _output "DoNotLock" false true)
        (set `PlayerController.bShowMouseCursor` true _returnvalue)))))

(event `self.ReceiveAnyDamage`
  (params (Damage :type "Float (single-precision)") (DamageType :type "DamageType Object Reference") (InstigatedBy :type "Controller Object Reference") (DamageCauser :type "Actor Object Reference"))
  (bind _returnvalue (`self.K2_GetActorLocation`))
  (`GameplayStatics.PlaySoundAtLocation` "/Game/Sounds/SC_Hurt.SC_Hurt" _returnvalue (struct) 1.0 1.0 0.0 null null null null)
  (`NiagaraFunctionLibrary.SpawnSystemAtLocation` "/Game/Particles/NS_Blood.NS_Blood" _returnvalue))

(event `/Game/Blueprints/Interfaces/BPI_Weapons.SetRightWeapon`
  (params (Class :type "Actor Class Reference"))
  (bind _righthandthrowable (`self.RightHandThrowable`))
  (bind _childactor (`ChildActorComponent.ChildActor` _righthandthrowable))
  (`ChildActorComponent.SetChildActorClass` _righthandthrowable Class)
  (`/Engine/EditorBlueprintResources/StandardMacros.IsValid` _childactor
    (:`Is Valid`
      (`self.SetOwner` _childactor self)
      (`PrimitiveComponent.SetRenderCustomDepth` (`self.GetComponentByClass` _childactor "/Script/Engine.StaticMeshComponent") false))))

(event `/Game/Blueprints/Interfaces/BPI_Weapons.SetLeftWeapon`
  (params (Class :type "Actor Class Reference"))
  (bind _lefthandthrowable (`self.LeftHandThrowable`))
  (bind _childactor (`ChildActorComponent.ChildActor` _lefthandthrowable))
  (`ChildActorComponent.SetChildActorClass` _lefthandthrowable Class)
  (`/Engine/EditorBlueprintResources/StandardMacros.IsValid` _childactor
    (:`Is Valid`
      (`self.SetOwner` _childactor self)
      (`PrimitiveComponent.SetRenderCustomDepth` (`self.GetComponentByClass` _childactor "/Script/Engine.StaticMeshComponent") false))))

(event `EnhancedInput|/Game/Data/Input/IA_Kick`
  (params (ActionValue :type Boolean) (ElapsedSeconds :type "Float (double-precision)") (TriggeredSeconds :type "Float (double-precision)") (InputAction :type "InputAction Object Reference" :default "/Game/Data/Input/IA_Kick.IA_Kick"))
  (bind _returnvalue (`SceneComponent.K2_GetComponentLocation` (`self.ChestCentre`)))
  (:`Triggered`
    (bind _outhits (`KismetSystemLibrary.CapsuleTraceMulti` _returnvalue (+ _returnvalue (* (`self.GetActorForwardVector`) 120.0)) 50.0 50.0 "TraceTypeQuery1"))
    (`ActionManager.ExecuteAction` (`self.ActionsManager`) (struct :`TagName` "Action.Kick"))
    (bind _results (`self.CorrectlyFilterHits` _outhits))
    (if (> (`KismetArrayLibrary.Array_Length` _results) 0)
      (`GameplayStatics.PlaySoundAtLocation` "/Game/Sounds/SC_Punch.SC_Punch" (`self.K2_GetActorLocation`) (struct) 1.0 1.0 0.0 null null null null))
    (for _array_element _results
      (`self.ProcessHit` _array_element false true))))

(event `/Game/Blueprints/Interfaces/BPI_Weapons.CallEnemyHit`
  (params (AttackType :type "EAttackType Enum" :default "LightAttack"))
  (`self.OnEnemyHit` "Throwable"))

(event `self.Interaction.OnComponentBeginOverlap`
  (params (OverlappedComponent :type "PrimitiveComponent Object Reference") (OtherActor :type "Actor Object Reference") (OtherComp :type "PrimitiveComponent Object Reference") (OtherBodyIndex :type Integer) (bFromSweep :type Boolean) (SweepResult :type "HitResult Structure (by ref)"))
  (bind _pickup (message `/Game/Blueprints/Interfaces/BPI_Pickup.IsPickup` OtherActor))
  (if _pickup
    (if (!= (`self.GetOwner` OtherActor) self)
      (`PrimitiveComponent.SetRenderCustomDepth` (`self.GetComponentByClass` OtherActor "/Script/Engine.StaticMeshComponent") true))))

(event `self.Interaction.OnComponentEndOverlap`
  (params (OverlappedComponent :type "PrimitiveComponent Object Reference") (OtherActor :type "Actor Object Reference") (OtherComp :type "PrimitiveComponent Object Reference") (OtherBodyIndex :type Integer))
  (bind _pickup (message `/Game/Blueprints/Interfaces/BPI_Pickup.IsPickup` OtherActor))
  (if _pickup
    (if (!= (`self.GetOwner` OtherActor) self)
      (`PrimitiveComponent.SetRenderCustomDepth` (`self.GetComponentByClass` OtherActor "/Script/Engine.StaticMeshComponent") false))))

(event `self.StatsComponent.OnStatisticReachedZero`
  (params (StatisticTag :type "GameplayTag Structure"))
  (bind _returnvalue (`GameplayStatics.GetPlayerController` 0))
  (if (== StatisticTag (struct :`TagName` "Stats.Health"))
    (`KismetSystemLibrary.Delay` 0.1)
    (`TimeDilationManager.PrepareDestroy` (`self.GetComponentByClass` (`GameplayStatics.GetGameMode`) "/Script/untitledfightgame.TimeDilationManager"))
    (`GameplayStatics.SetGamePaused` true)
    (bind _foundwidgets (`WidgetBlueprintLibrary.GetAllWidgetsOfClass` "/Game/Blueprints/UI/Core/WBP_Base.WBP_Base_C"))
    (bind _output (`|GetArrayItem` _foundwidgets))
    (`CommonActivatableWidgetContainerBase.BP_AddWidget` (`/Game/Blueprints/UI/Core/WBP_Base.PauseStack` _output) "/Game/Blueprints/UI/Game/WBP_Death.WBP_Death_C")
    (`WidgetBlueprintLibrary.SetInputMode_GameAndUIEx` _returnvalue _output "DoNotLock" false)
    (set `PlayerController.bShowMouseCursor` true _returnvalue)))

(event `self.StatsComponent.OnStatisticUpdated`
  (params (StatisticTag :type "GameplayTag Structure"))
  (bind _returnvalue_currentvalue (break `StatisticInformation` (`StatisticsComponent.GetStatInfoByTag` (`self.StatsComponent`) (struct :`TagName` "Stats.Health"))))
  (if (== StatisticTag (struct :`TagName` "Stats.Health"))
    (bind _difficulty (message `/Game/Blueprints/Interfaces/BPI_Difficulty.GetDifficulty` (`GameplayStatics.GetGameInstance`)))
    (if (`|EnumInequality` _difficulty "NewEnumerator1")
      (if (< _returnvalue_currentvalue (`self.LastHealth`))
        (set `self.LastHealth` _returnvalue_currentvalue)
        (`KismetSystemLibrary.K2_ClearAndInvalidateTimerHandle` (`self.HealingTimer`))
        (bind _returnvalue (`KismetSystemLibrary.K2_SetTimerDelegate` (delegate `CustomEvent_0`) 1.0 true false 3.0))
        (set `self.HealingTimer` _returnvalue)
        (else
          (set `self.LastHealth` _returnvalue_currentvalue))))))

(event `CustomEvent_0`
  (bind _statscomponent (`self.StatsComponent`))
  (bind (_returnvalue_currentvalue _returnvalue_maxvalue) (break `StatisticInformation` (`StatisticsComponent.GetStatInfoByTag` _statscomponent (struct :`TagName` "Stats.Health"))))
  (`StatisticsComponent.ModifyCurrentValueOfStatistic` _statscomponent (struct :`TagName` "Stats.Health") 10.0)
  (if (== _returnvalue_currentvalue _returnvalue_maxvalue)
    (`KismetSystemLibrary.K2_ClearAndInvalidateTimerHandle` (`self.HealingTimer`))))

(fn `CorrectlyFilterHits`
  (params (Hits :type "Array of HitResult Structure"))
  (returns (Results :type "Array of HitResult Structure"))
  (locals (TempArray :type "Array of HitResult Structure") (TempArrayActors :type "Array of Actor Object Reference") (TempActor :type "Actor Object Reference"))
  (for _array_element Hits
    (set `local.TempActor` (`.HitActor` (`GameplayStatics.BreakHitResult` _array_element)))
    (if (not (`KismetArrayLibrary.Array_Contains` (`local.TempArrayActors`) (`local.TempActor`)))
      (`KismetArrayLibrary.Array_Add` (`local.TempArray`) _array_element)
      (`KismetArrayLibrary.Array_Add` (`local.TempArrayActors`) (`local.TempActor`))))
  (return (`local.TempArray`)))

(fn `HaveLeftWeapon`
  (returns (HasLeftWeapon :type Boolean))
  (return (`KismetSystemLibrary.IsValid` (`ChildActorComponent.ChildActor` (`self.LeftHandThrowable`)))))

(fn `HaveRightWeapon`
  (returns (HasRightWeapon :type Boolean))
  (return (`KismetSystemLibrary.IsValid` (`ChildActorComponent.ChildActor` (`self.RightHandThrowable`)))))

(fn `IsEnemy`
  (returns (Enemy :type Boolean))
  (return false))

(fn `IsPlayerCharacter`
  (returns (Character :type Boolean))
  (return true))

(fn `ProcessHit`
  (params (Hit :type "HitResult Structure") (IsHeavyHit :type Boolean) (IsKick :type Boolean))
  (bind (_bblockinghit _binitialoverlap _time _distance _location _impactpoint _normal _impactnormal _physmat _hitactor) (`GameplayStatics.BreakHitResult` Hit))
  (bind _isheavyhit (`local.IsHeavyHit`))
  (bind _returnvalue (`EventsManager.IsEventActive` (`self.GetComponentByClass` (`GameplayStatics.GetGameMode`) "/Script/untitledfightgame.EventsManager") (`BlueprintGameplayTagLibrary.MakeLiteralGameplayTag` (struct :`TagName` "Events.Rage"))))
  (`/Engine/EditorBlueprintResources/StandardMacros.IsValid` _hitactor
    (:`Is Valid`
      (if (`Actor.bCanBeDamaged` _hitactor)
        (bind _enemy (message `/Game/Blueprints/Interfaces/BPI_Character.IsEnemy` _hitactor))
        (if _enemy
          (`self.OnEnemyHit` (select `bool` (`local.IsKick`) :`false` (select `bool` _isheavyhit :`false` "LightAttack" :`true` "HeavyAttack" :!type "EAttackType Enum") :`true` "Kick")))
        (`GameplayStatics.ApplyDamage` _hitactor (select `bool` (`local.IsKick`) :`false` (* 25.0 (`KismetMathLibrary.SelectFloat` 2.0 1.0 _returnvalue)) :`true` (* 10.0 (`KismetMathLibrary.SelectFloat` 2.0 1.0 _returnvalue)) :!type "Float (single-precision)") (`self.GetController`) self (select `bool` (`local.IsKick`) :`false` (select `bool` _isheavyhit :`false` "/Game/Data/BP_LightAttack.BP_LightAttack_C" :`true` "/Game/Data/BP_HeavyAttack.BP_HeavyAttack_C" :!type "DamageType Class Reference") :`true` "/Game/Data/BP_Kick.BP_Kick_C"))))))

(fn `ThrowWeapon`
  (params (`Right?` :type Boolean))
  (bind _returnvalue (`SceneComponent.K2_GetComponentLocation` (`self.ChestCentre1`)))
  (bind _returnvalue_2 (`SceneComponent.K2_GetComponentLocation` (`self.ChestCentre2`)))
  (bind _returnvalue_3 (`self.GetComponentByClass` (`ChildActorComponent.ChildActor` (`self.LeftHandThrowable`)) "/Script/Engine.StaticMeshComponent"))
  (bind _returnvalue_4 (`self.GetComponentByClass` (`ChildActorComponent.ChildActor` (`self.RightHandThrowable`)) "/Script/Engine.StaticMeshComponent"))
  (if `Right?`
    (bind _returnvalue_5 (`|SpawnActorFromClass` "/Game/Blueprints/Throwables/Core/BP_Projectile.BP_Projectile_C" (`KismetMathLibrary.MakeTransform` (`SceneComponent.K2_GetComponentLocation` (`self.RightHandThrowable`)) (`KismetMathLibrary.FindLookAtRotation` _returnvalue (+ _returnvalue (* (`SceneComponent.GetForwardVector` (`self.Camera`)) 500.0)))) "AlwaysSpawn" "MultiplyWithRoot" null null))
    (`/Engine/EditorBlueprintResources/StandardMacros.IsValid` _returnvalue_5 ; If not valid, it's a good chance that it already\nbroke as it was colliding with something.
      (:`Is Valid`
        (bind _staticmesh (`/Game/Blueprints/Throwables/Core/BP_Projectile.StaticMesh` _returnvalue_5))
        (`StaticMeshComponent.SetStaticMesh` _staticmesh (`StaticMeshComponent.StaticMesh` _returnvalue_4))
        (`PrimitiveComponent.SetMaterial` _staticmesh 0 (`PrimitiveComponent.GetMaterial` _returnvalue_4 0)))
      (:`Is Not Valid`
        _))
    (`/Game/Blueprints/Interfaces/BPI_Weapons.SetRightWeapon` null)
    (`ActionManager.ExecuteAction` (`self.ActionsManager`) (struct :`TagName` "Action.LightRight"))
    (else
      (bind _returnvalue_6 (`|SpawnActorFromClass` "/Game/Blueprints/Throwables/Core/BP_Projectile.BP_Projectile_C" (`KismetMathLibrary.MakeTransform` (`SceneComponent.K2_GetComponentLocation` (`self.LeftHandThrowable`)) (`KismetMathLibrary.FindLookAtRotation` _returnvalue_2 (+ _returnvalue_2 (* (`SceneComponent.GetForwardVector` (`self.Camera`)) 80.0)))) "AlwaysSpawn" "MultiplyWithRoot" null null))
      (`/Engine/EditorBlueprintResources/StandardMacros.IsValid` _returnvalue_6
        (:`Is Valid`
          (bind _staticmesh_2 (`/Game/Blueprints/Throwables/Core/BP_Projectile.StaticMesh` _returnvalue_6))
          (`StaticMeshComponent.SetStaticMesh` _staticmesh_2 (`StaticMeshComponent.StaticMesh` _returnvalue_3))
          (`PrimitiveComponent.SetMaterial` _staticmesh_2 0 (`PrimitiveComponent.GetMaterial` _returnvalue_3 0)))
        (:`Is Not Valid`
          _))
      (`/Game/Blueprints/Interfaces/BPI_Weapons.SetLeftWeapon` null)
      (`ActionManager.ExecuteAction` (`self.ActionsManager`) (struct :`TagName` "Action.LightLeft")))))

(fn `UserConstructionScript`)