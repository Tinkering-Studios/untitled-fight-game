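; Enemy character Blueprint for melee combat, handling its punches, hit reactions and death.
; ActionsManager action tags trigger left or right, light or heavy capsule traces, which apply equal damage with differing damage types.
; Damage received launches it along the player's forward vector, scaled by damage type.
; StatsComponent health updates spawn blood; zero health stops AI logic and replaces the actor with an explosion and an impulse-driven ragdoll.
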(event `self.ReceiveBeginPlay`
  (bind _returnvalue_currentvalue (break `StatisticInformation` (`StatisticsComponent.GetStatInfoByTag` (`self.StatsComponent`) (struct :`TagName` "Stats.Health"))))
  (set `self.LastHealth` _returnvalue_currentvalue))

(event `LightAttack`
  (params (IsRight :type Boolean))
  (bind _returnvalue (`SceneComponent.K2_GetComponentLocation` (`self.ChestCentre1`)))
  (bind _returnvalue_2 (`SceneComponent.K2_GetComponentLocation` (`self.ChestCentre2`)))
  (if IsRight
    (bind _outhit (`KismetSystemLibrary.CapsuleTraceSingle` _returnvalue (+ _returnvalue (* (`self.GetActorForwardVector`) 80.0)) 50.0 25.0 "TraceTypeQuery1"))
    (`self.ProcessHit` _outhit)
    (else
      (bind _outhit_2 (`KismetSystemLibrary.CapsuleTraceSingle` _returnvalue_2 (+ _returnvalue_2 (* (`self.GetActorForwardVector`) 80.0)) 50.0 50.0 "TraceTypeQuery1"))
      (`self.ProcessHit` _outhit_2))))

(event `HeavyAttack`
  (params (IsRight :type Boolean))
  (bind _returnvalue (`SceneComponent.K2_GetComponentLocation` (`self.ChestCentre1`)))
  (bind _returnvalue_2 (`SceneComponent.K2_GetComponentLocation` (`self.ChestCentre2`)))
  (if IsRight
    (bind _outhit (`KismetSystemLibrary.CapsuleTraceSingle` _returnvalue (+ _returnvalue (* (`self.GetActorForwardVector`) 80.0)) 50.0 25.0 "TraceTypeQuery1"))
    (`self.ProcessHit` _outhit true)
    (else
      (bind _outhit_2 (`KismetSystemLibrary.CapsuleTraceSingle` _returnvalue_2 (+ _returnvalue_2 (* (`self.GetActorForwardVector`) 80.0)) 50.0 50.0 "TraceTypeQuery1"))
      (`self.ProcessHit` _outhit_2 true))))

(event `self.ReceiveAnyDamage`
  (params (Damage :type "Float (single-precision)") (DamageType :type "DamageType Object Reference") (InstigatedBy :type "Controller Object Reference") (DamageCauser :type "Actor Object Reference"))
  (bind _returnvalue (== (`GameplayStatics.GetObjectClass` DamageType) "/Game/Data/BP_LightAttack.BP_LightAttack_C"))
  (bind (_returnvalue_x _returnvalue_y _returnvalue_z) (`KismetMathLibrary.BreakVector` (* (`self.GetActorForwardVector` (`GameplayStatics.GetPlayerCharacter` 0)) (`KismetMathLibrary.SelectFloat` 1000.0 300.0 _returnvalue))))
  (`MovementComponent.StopMovementImmediately` (`self.CharacterMovement`))
  (`self.LaunchCharacter` (`KismetMathLibrary.MakeVector` _returnvalue_x _returnvalue_y (+ _returnvalue_z (`KismetMathLibrary.SelectFloat` 200.0 300.0 _returnvalue))))
  (`GameplayStatics.PlaySoundAtLocation` "/Game/Sounds/SC_Hurt.SC_Hurt" (`self.K2_GetActorLocation`) (struct) 1.0 1.0 0.0 null null null null))

(event `self.StatsComponent.OnStatisticReachedZero`
  (params (StatisticTag :type "GameplayTag Structure"))
  (if (== StatisticTag (struct :`TagName` "Stats.Health"))
    (`|SpawnActorFromClass` "/Game/Blueprints/Effects/BP_BloodExplosion.BP_BloodExplosion_C" (`KismetMathLibrary.MakeTransform` (`SceneComponent.K2_GetComponentLocation` (`self.Sphere`))) "AlwaysSpawn" "MultiplyWithRoot" null null)
    (`GameplayStatics.PlaySoundAtLocation` "/Game/Sounds/SC_Hurt.SC_Hurt" (`self.K2_GetActorLocation`) (struct) 1.0 0.75 0.0 null null null null)
    (`MovementComponent.StopMovementImmediately` (`self.CharacterMovement`))
    (bind _asmain_aicontroller (cast `MainAIController` (`self.GetController`)))
    (`BrainComponent.StopLogic` (`AIController.BrainComponent` _asmain_aicontroller) "Death")
    (bind _returnvalue (`|SpawnActorFromClass` "/Game/Blueprints/Enemies/Ragdoll.Ragdoll_C" (`SceneComponent.K2_GetComponentToWorld` (`self.Mesh`)) "Undefined" "MultiplyWithRoot" null null))
    (`PrimitiveComponent.AddRadialImpulse` (`/Game/Blueprints/Enemies/Ragdoll.SkeletalMesh` _returnvalue) (`self.K2_GetActorLocation` (`GameplayStatics.GetPlayerCharacter` 0)) 500.0 75000.0 "RIF_Constant" false)
    (`self.K2_DestroyActor`)))

(event `self.StatsComponent.OnStatisticUpdated`
  (params (StatisticTag :type "GameplayTag Structure"))
  (bind _returnvalue_currentvalue (break `StatisticInformation` (`StatisticsComponent.GetStatInfoByTag` (`self.StatsComponent`) (`BlueprintGameplayTagLibrary.MakeLiteralGameplayTag` (struct :`TagName` "Stats.Health")))))
  (if (== StatisticTag (struct :`TagName` "Stats.Health"))
    (if (> (`self.LastHealth`) 0.0)
      (set `self.LastHealth` _returnvalue_currentvalue)
      (`NiagaraFunctionLibrary.SpawnSystemAtLocation` "/Game/Particles/NS_Blood.NS_Blood" (`SceneComponent.K2_GetComponentLocation` (`self.Sphere`))))))

(event `self.ActionsManager.OnActionStarted`
  (params (ActionTag :type "GameplayTag Structure"))
  (`|SwitchGameplayTag` ActionTag
    (:`Action.HeavyLeft`
      (`self.HeavyAttack` false))
    (:`Action.HeavyRight`
      (`self.HeavyAttack` true))
    (:`Action.LightLeft`
      (`self.LightAttack` false))
    (:`Action.LightRight`
      (`self.LightAttack` true))))

(fn `IsEnemy`
  (returns (Enemy :type Boolean))
  (return true))

(fn `IsPlayerCharacter`
  (returns (Character :type Boolean))
  (return false))

(fn `ProcessHit`
  (params (Hit :type "HitResult Structure") (IsHeavyHit :type Boolean))
  (bind (_bblockinghit _binitialoverlap _time _distance _location _impactpoint _normal _impactnormal _physmat _hitactor) (`GameplayStatics.BreakHitResult` Hit))
  (`/Engine/EditorBlueprintResources/StandardMacros.IsValid` _hitactor
    (:`Is Valid`
      (`GameplayStatics.PlaySoundAtLocation` "/Game/Sounds/SC_Punch.SC_Punch" (`self.K2_GetActorLocation`) (struct) 1.0 1.0 0.0 null null null null)
      (if (`Actor.bCanBeDamaged` _hitactor)
        (`GameplayStatics.ApplyDamage` _hitactor 10.0 null null (select `bool` (`local.IsHeavyHit`) :`false` "/Game/Data/BP_LightAttack.BP_LightAttack_C" :`true` "/Game/Data/BP_HeavyAttack.BP_HeavyAttack_C" :!type "DamageType Class Reference"))))))

(fn `UserConstructionScript`)