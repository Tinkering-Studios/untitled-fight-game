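; Slot machine actor that spins three reels when something overlaps its TestBox and plays a sound when all three results match.
; On overlap it draws a result per reel from RandomRot, then plays the Rotate timeline.
; Separate timeline tracks drive SlotRotation, which lerps each reel's pitch through many turns.
; A reel whose alpha reaches one snaps to its drawn pitch, and the match check runs when the timeline finishes.
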(event `self.ReceiveBeginPlay`
  (set `self.Original rotation` (`SceneComponent.K2_GetComponentRotation` (`self.Slot1`))))

(event `self.TestBox.OnComponentBeginOverlap`
  (params (OverlappedComponent :type "PrimitiveComponent Object Reference") (OtherActor :type "Actor Object Reference") (OtherComp :type "PrimitiveComponent Object Reference") (OtherBodyIndex :type Integer) (bFromSweep :type Boolean) (SweepResult :type "HitResult Structure (by ref)"))
  (bind (_original_rotation_roll _original_rotation_pitch _original_rotation_yaw) (`KismetMathLibrary.BreakRotator` (`self.Original rotation`)))
  (bind (_original_rotation_roll_2 _original_rotation_pitch_2 _original_rotation_yaw_2) (`KismetMathLibrary.BreakRotator` (`self.Original rotation`)))
  (bind (_original_rotation_roll_3 _original_rotation_pitch_3 _original_rotation_yaw_3) (`KismetMathLibrary.BreakRotator` (`self.Original rotation`)))
  (bind _rand1_0 (`self.Rand1_0`))
  (set `self.Rand1` (`self.RandomRot`))
  (set `self.Rand1_0` (`self.RandomRot`))
  (set `self.Rand1_1` (`self.RandomRot`))
  (bind (_direction _3 _3_5 _4) (`Timeline|Rotate` :!via `PlayFromStart`)
    (:`Update`
      (bind _end (`self.SlotRotation` (`self.Slot3`) _4))
      (if _end
        (`SceneComponent.K2_SetWorldRotation` (`self.Slot3`) (`KismetMathLibrary.MakeRotator` _original_rotation_roll_2 (`self.Rand1`) _original_rotation_yaw_2) false false)
        (else
          (bind _end_2 (`self.SlotRotation` (`self.Slot2`) _3_5))
          (if _end_2
            (`SceneComponent.K2_SetWorldRotation` (`self.Slot2`) (`KismetMathLibrary.MakeRotator` _original_rotation_roll_3 (`self.Rand1_0`) _original_rotation_yaw_3) false false)
            (else
              (bind _end_3 (`self.SlotRotation` (`self.Slot1`) _3))
              (if _end_3
                (`SceneComponent.K2_SetWorldRotation` (`self.Slot1`) (`KismetMathLibrary.MakeRotator` _original_rotation_roll (`self.Rand1_1`) _original_rotation_yaw) false false)))))))
    (:`Finished`
      (if (and (== (`self.Rand1`) _rand1_0) (== _rand1_0 (`self.Rand1_1`)))
        (`GameplayStatics.PlaySound2D` "/Game/Sounds/681107__simbakademzeb1__es_slot-machine-41-sfx-producer.681107__simbakademzeb1__es_slot-machine-41-sfx-producer" 1.0 1.0 0.0 null null)))))

(fn `SlotRotation`
  (params (Mesh :type "SceneComponent Object Reference") (Alpha :type "Float (double-precision)"))
  (returns (End :type Boolean))
  (bind (_original_rotation_roll _original_rotation_pitch _original_rotation_yaw) (`KismetMathLibrary.BreakRotator` (`self.Original rotation`)))
  (`SceneComponent.K2_SetWorldRotation` Mesh (`KismetMathLibrary.RLerp` (`self.Original rotation`) (`KismetMathLibrary.MakeRotator` _original_rotation_roll 8000.0 _original_rotation_yaw) Alpha) false false)
  (return (== Alpha 1.0)))

(fn `UserConstructionScript`)