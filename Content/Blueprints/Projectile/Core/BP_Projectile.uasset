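; BP_Projectile is a thrown-weapon projectile that damages what it overlaps and then destroys itself.
; On overlap it skips the player character, actors of its own class, and actors parented to throwable pickups, the player or other projectiles.
; A valid hit plays a sound, sends the player an enemy-hit message, and applies fixed throwable-type damage credited to the player.
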(event `self.ReceiveActorBeginOverlap`
  (params (OtherActor :type "Actor Object Reference"))
  (bind _returnvalue (`GameplayStatics.GetPlayerCharacter` 0))
  (bind _returnvalue_2 (`GameplayStatics.GetObjectClass` (`self.GetParentActor` OtherActor)))
  (if (!= OtherActor (`GameplayStatics.GetPlayerCharacter` 0))
    (if (and (!= _returnvalue_2 "/Game/Blueprints/Throwables/Core/BP_PickupThrowable.BP_PickupThrowable_C") (!= _returnvalue_2 "/Game/Blueprints/Core/BP_PlayerCharacter.BP_PlayerCharacter_C") (!= _returnvalue_2 "BP_Projectile_C") (!= (`GameplayStatics.GetObjectClass` self) (`GameplayStatics.GetObjectClass` OtherActor)))
      (`GameplayStatics.PlaySoundAtLocation` (`self.HitSound`) (`self.K2_GetActorLocation`) (struct) 1.0 1.0 0.0 null null null null)
      (message `/Game/Blueprints/Interfaces/BPI_Weapons.CallEnemyHit` _returnvalue "Throwable")
      (`GameplayStatics.ApplyDamage` OtherActor 25.0 (`Pawn.GetController` _returnvalue) _returnvalue "/Game/Data/BP_Throwable.BP_Throwable_C")
      (`self.K2_DestroyActor`))))

(fn `UserConstructionScript`)