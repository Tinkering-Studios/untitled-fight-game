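; BP_BloodProjectile is a blood effect projectile that leaves a puddle when it hits a suitable surface.
; On BeginPlay it sets a random initial speed on its ProjectileMovement and activates it.
; When its Sphere overlaps an actor tagged "Bloodable", it spawns a BP_BloodPuddle at its own location with that actor's rotation, then destroys itself.
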(event `self.ReceiveBeginPlay`
  (bind _projectilemovement (`self.ProjectileMovement`))
  (set `ProjectileMovementComponent.InitialSpeed` (`KismetMathLibrary.RandomFloatInRange` 400.0 800.0) _projectilemovement)
  (`ActorComponent.Activate` _projectilemovement true))

(event `self.Sphere.OnComponentBeginOverlap`
  (params (OverlappedComponent :type "PrimitiveComponent Object Reference") (OtherActor :type "Actor Object Reference") (OtherComp :type "PrimitiveComponent Object Reference") (OtherBodyIndex :type Integer) (bFromSweep :type Boolean) (SweepResult :type "HitResult Structure (by ref)"))
  (if (`self.ActorHasTag` OtherActor "Bloodable")
    (`|SpawnActorFromClass` "/Game/Blueprints/WorldObjects/BP_BloodPuddle.BP_BloodPuddle_C" (`KismetMathLibrary.MakeTransform` (`self.K2_GetActorLocation`) (`self.K2_GetActorRotation` OtherActor)) "AlwaysSpawn" "MultiplyWithRoot" null null)
    (`self.K2_DestroyActor`)))

(fn `UserConstructionScript`)