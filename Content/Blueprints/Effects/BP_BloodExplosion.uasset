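; BP_BloodExplosion is a gore effect that sprays a burst of BP_BloodProjectile actors when it begins play.
; A loop with a random count spawns the projectiles at the actor's location, ignoring collisions.
; Each projectile is rotated to face one of four Sphere components picked at random, so the spheres serve as aim markers that define the spray directions.
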(event `self.ReceiveBeginPlay`
  (bind _returnvalue (`self.K2_GetActorLocation`))
  (for _ (range (+ (`KismetMathLibrary.RandomIntegerInRange` 2 6) 1))
    (`|SpawnActorFromClass` "/Game/Blueprints/Effects/BP_BloodProjectile.BP_BloodProjectile_C" (`KismetMathLibrary.MakeTransform` _returnvalue (`KismetMathLibrary.FindLookAtRotation` _returnvalue (`SceneComponent.K2_GetComponentLocation` (select `int` (`KismetMathLibrary.RandomIntegerInRange` 0 3) :`0` (`self.Sphere`) :`1` (`self.Sphere1`) :`2` (`self.Sphere2`) :`3` (`self.Sphere3`) :!type "SceneComponent Object Reference")))) "AlwaysSpawn" "MultiplyWithRoot" null null)))

(fn `UserConstructionScript`)