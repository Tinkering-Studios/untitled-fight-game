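; BP_PickupThrowable is a throwable actor that gets picked up when damaged while it has no owner.
; It reads the damage causer's current ActionManager action and branches on the Light Left or Light Right gameplay tag.
; If that hand has no weapon, it passes its class to the causer and destroys itself.
; Both branches call SetLeftWeaponMessage, even though the right branch checks the right hand.
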(event `self.ReceiveAnyDamage`
  (params (Damage :type "Float (single-precision)") (DamageType :type "DamageType Object Reference") (InstigatedBy :type "Controller Object Reference") (DamageCauser :type "Actor Object Reference"))
  (bind _returnvalue (`GameplayStatics.GetObjectClass` self))
  (`/Engine/EditorBlueprintResources/StandardMacros.IsValid` DamageCauser
    (:`Is Valid`
      (`/Engine/EditorBlueprintResources/StandardMacros.IsValid` (`self.GetOwner`)
        (:`Is Not Valid`
          (bind _returnvalue_2 (`ActionManager.GetCurrentAction` (`self.GetComponentByClass` DamageCauser "/Script/untitledfightgame.ActionManager")))
          (`|SwitchGameplayTag` _returnvalue_2
            (:`Action.LightLeft`
              (bind _hasleftweapon (message `/Game/Blueprints/Interfaces/BPI_Weapons.HaveLeftWeapon` DamageCauser))
              (if (not _hasleftweapon)
                (message `/Game/Blueprints/Interfaces/BPI_Weapons.SetLeftWeapon` DamageCauser _returnvalue)
                (`self.K2_DestroyActor`)))
            (:`Action.LightRight`
              (bind _hasrightweapon (message `/Game/Blueprints/Interfaces/BPI_Weapons.HaveRightWeapon` DamageCauser))
              (if (not _hasrightweapon)
                (message `/Game/Blueprints/Interfaces/BPI_Weapons.SetLeftWeapon` DamageCauser _returnvalue)
                (`self.K2_DestroyActor`)))))))))

(fn `UserConstructionScript`)