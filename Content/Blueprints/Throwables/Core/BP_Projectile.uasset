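; Base actor for thrown projectiles that break on overlap and damage enemies.
; Overlap ignores the player, pickup throwables and other projectiles; otherwise it plays impact sound and particles, then destroys itself.
; Targets identified as enemies through a message call take fixed damage credited to the player, who is notified of the hit.
; Impact effects are picked from the mesh's material, with special glass and card variants overriding the defaults.
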(event `self.ReceiveActorBeginOverlap`
  (params (OtherActor :type "Actor Object Reference"))
  (bind _returnvalue (`GameplayStatics.GetPlayerCharacter` 0))
  (bind _returnvalue_2 (`self.K2_GetActorLocation`))
  (bind _returnvalue_3 (`GameplayStatics.GetObjectClass` (`self.GetParentActor` OtherActor)))
  (if (!= OtherActor (`GameplayStatics.GetPlayerCharacter` 0))
    (if (and (!= _returnvalue_3 "/Game/Blueprints/Throwables/Core/BP_PickupThrowable.BP_PickupThrowable_C") (!= _returnvalue_3 "/Game/Blueprints/Core/BP_PlayerCharacter.BP_PlayerCharacter_C") (!= _returnvalue_3 "BP_Projectile_C") (!= (`GameplayStatics.GetObjectClass` self) (`GameplayStatics.GetObjectClass` OtherActor)))
      (`GameplayStatics.PlaySoundAtLocation` (`self.GetHitSound`) _returnvalue_2 (struct) 1.0 1.0 0.0 null null null null)
      (`NiagaraFunctionLibrary.SpawnSystemAtLocation` (`self.GetParticle`) _returnvalue_2 (struct) (0.5 0.5 0.5))
      (bind _enemy (message `/Game/Blueprints/Interfaces/BPI_Character.IsEnemy` OtherActor))
      (if _enemy
        (message `/Game/Blueprints/Interfaces/BPI_Weapons.CallEnemyHit` _returnvalue "Throwable")
        (`GameplayStatics.ApplyDamage` OtherActor 25.0 (`Pawn.GetController` _returnvalue) _returnvalue "/Game/Data/BP_Throwable.BP_Throwable_C"))
      (`self.K2_DestroyActor`))))

(fn `GetHitSound`
  (returns (Sound :type "SoundBase Object Reference"))
  (return (select `bool` (== (`PrimitiveComponent.GetMaterial` (`self.StaticMesh`) 0) "/Game/Materials/MI_StrongGlass.MI_StrongGlass") :`false` (`self.HitSound`) :`true` "/Game/Sounds/SC_Glass.SC_Glass")))

(fn `GetParticle`
  (returns (Sound :type "NiagaraSystem Object Reference"))
  (return (select `bool` (== (`PrimitiveComponent.GetMaterial` (`self.StaticMesh`) 0) "/Game/Materials/MI_StrongGlass.MI_StrongGlass") :`false` (select `bool` (== (`PrimitiveComponent.GetMaterial` (`self.StaticMesh`) 0) "/Game/Materials/M_Cards.M_Cards") :`false` (`self.Particle`) :`true` "/Game/Particles/NS_CardsBreak.NS_CardsBreak") :`true` "/Game/Particles/Ns_Glass.Ns_Glass")))

(fn `UserConstructionScript`)