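; BP_VendingItem is a throwable vending item that appears as one of several food models.
; Its construction script picks a random food mesh for the StaticMesh component, then runs the parent construction script.
; The event graph holds only disabled default events, so this Blueprint adds no runtime logic of its own.
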(fn `UserConstructionScript`
  (`StaticMeshComponent.SetStaticMesh` (`self.StaticMesh`) (select `int` (`KismetMathLibrary.RandomIntegerInRange` 0 4) :`0` "/Game/Models/Food/food_FOOD.food_FOOD" :`1` "/Game/Models/Food/food_FOOD_006.food_FOOD_006" :`2` "/Game/Models/Food/food_FOOD_016.food_FOOD_016" :`3` "/Game/Models/Food/food_FOOD_017.food_FOOD_017" :`4` "/Game/Models/Food/food_FOOD_018.food_FOOD_018" :!type "StaticMesh Object Reference"))
  (`parent.UserConstructionScript`))